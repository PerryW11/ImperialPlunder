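; BP_KeyDoor is a locked door that opens when the player pawn has collected enough keys.
; Overlapping its Box casts the actor to DefaultPawn_BP, then checks and deducts RequiredNumberOfKeys from NumberOfKeys.
; The DoorMovement timeline then sets the Door's relative location from a rotator lerped toward TargetRotation's direction and converted to an X vector, so it changes position rather than rotation.
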(event OnComponentBeginOverlap(Box)
  (params (OverlappedComponent :type Primitive%20Component%20Object%20Reference) (OtherActor :type Actor%20Object%20Reference) (OtherComp :type Primitive%20Component%20Object%20Reference) (OtherBodyIndex :type Integer) (bFromSweep :type Boolean) (SweepResult :type Hit%20Result%20Structure%20%28by%20ref%29))
  (bind _requirednumberofkeys (Variables|Default|GetRequiredNumberOfKeys))
  (bind _asdefault_pawn_bp (Utilities|Casting|CastToDefaultPawn_BP OtherActor))
  (if (>= (Variables|/Game/DefaultPawn_BP.DefaultPawn_BP_C|GetNumberOfKeys _asdefault_pawn_bp) _requirednumberofkeys)
    (Variables|/Game/DefaultPawn_BP.DefaultPawn_BP_C|SetNumberOfKeys _asdefault_pawn_bp (- (Variables|/Game/DefaultPawn_BP.DefaultPawn_BP_C|GetNumberOfKeys _asdefault_pawn_bp) _requirednumberofkeys))
    (bind _alpha (Timeline|DoorMovement Play)
      (:Update
        (Transformation|SetRelativeLocation (Variables|Default|GetDoor) (Math|Rotator|GetRotationXVector (Math|Rotator|Lerp(Rotator) "0, 0, 0" (Math|Conversions|RotationFromXVector (Variables|Default|GetTargetRotation)) _alpha)) false false)))))

(event EventBeginPlay)

(event Collision|EventActorBeginOverlap
  (params (OtherActor :type Actor%20Object%20Reference)))

(event EventTick
  (params (DeltaSeconds :type Float%20%28single-precision%29)))

(fn ConstructionScript)